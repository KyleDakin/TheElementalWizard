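; Wood is a game object that reacts to being hit by fire with an explosion effect and optional self-destruction.
; OnFireHit prints a debug message, waits a configurable delay, then spawns the P_Explosion emitter attached to its ParticlePos component.
; If DestroyAfterTrig is set, it destroys the actor after a second configurable delay.
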(event EventBeginPlay
  (|CallParentFunction) ; This node is disabled and will not be called.\nDrag off pins to build functionality.
)

(event Collision|EventActorBeginOverlap
  (params (OtherActor :type Actor%20Object%20Reference))
  (|CallParentFunction OtherActor) ; This node is disabled and will not be called.\nDrag off pins to build functionality.
)

(event EventTick
  (params (DeltaSeconds :type Float%20%28single-precision%29))
  (|CallParentFunction DeltaSeconds) ; This node is disabled and will not be called.\nDrag off pins to build functionality.
)

(event EventOnFireHit
  (Development|PrintString "Wood On Fire")
  (Utilities|FlowControl|Delay (Variables|Default|GetDelayToTrig))
  (Utilities|FlowControl|Sequence
    (:then_0
      (Effects|SpawnEmitterAttached "/Game/StarterContent/Particles/P_Explosion.P_Explosion" (Variables|Default|GetParticlePos) "None"))
    (:then_1
      (if (Variables|Default|GetbDestroyAfterTrig)
        (Utilities|FlowControl|Delay (Variables|Default|GetDelayToDestroy))
        (Actor|DestroyActor)))))

(fn ConstructionScript
  (|CallParentFunction))