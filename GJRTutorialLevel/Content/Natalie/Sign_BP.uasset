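; Sign_BP is a readable sign that shows a dialogue on screen when interacted with.
; Its Interact event runs a FlipFlop: the first use creates a Dialogue widget for the first player controller and adds it to the viewport.
; The next use removes that stored widget from its parent, so repeated interactions toggle the dialogue on and off.
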(event EventInteract
  (params (Actor :type First%20Person%20Character%20Object%20Reference))
  (Variables|Default|SetMyDialogueWid (Variables|Default|GetMyDialogueWid))
  (Utilities|FlowControl|FlipFlop
    (:A
      (bind _returnvalue (UserInterface|CreateWidget "/Game/Natalie/Dialogue.Dialogue_C" (Game|GetPlayerController 0)))
      (bind _output_get (Variables|Default|SetMyDialogueWid _returnvalue))
      (UserInterface|Viewport|AddtoViewport _output_get 0)
      (Variables|Default|SetMyText (Variables|Default|GetMyText)))
    (:B
      (Widget|RemovefromParent (Variables|Default|GetMyDialogueWid))
      (Variables|Default|SetDialogueWidget 0))))

(fn ConstructionScript)